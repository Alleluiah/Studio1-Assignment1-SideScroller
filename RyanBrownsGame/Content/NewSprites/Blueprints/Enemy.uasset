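; Paper2D-style enemy that patrols back and forth along world X and restarts play on touching the player character, Dave.
; Tick feeds slow movement input and rotates the sprite to match a direction boolean, which a Delay in Tick flips every few seconds.
; A capsule hit with Dave fires once, playing a death sound at the world origin and opening Level1 after a short delay.
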(event OnComponentHit(CapsuleComponent)
  (params (HitComponent :type Primitive%20Component%20Object%20Reference) (OtherActor :type Actor%20Object%20Reference) (OtherComp :type Primitive%20Component%20Object%20Reference) (NormalImpulse :type Vector :default "0, 0, 0") (Hit :type Hit%20Result%20Structure%20%28by%20ref%29))
  (Utilities|Casting|CastToDave OtherActor)
  (Utilities|FlowControl|DoOnce false
    (:Completed
      (Audio|PlaySoundatLocation "/Game/NewSprites/Audio/death_noise.death_noise" "0, 0, 0")
      (Utilities|FlowControl|Delay 1.0)
      (Game|OpenLevel(byName) "Level1"))))

(event EventBeginPlay)

(event Collision|EventActorBeginOverlap
  (params (OtherActor :type Actor%20Object%20Reference)))

(event EventTick
  (params (DeltaSeconds :type Float%20%28single-precision%29))
  (bind _sprite (Variables|Default|GetSprite))
  (if (Variables|Default|GetNewVar_0)
    (Transformation|SetWorldRotation _sprite "0,180.000000, 0" false false)
    (Pawn|Input|AddMovementInput "0.200000, 0, 0" 1.0 false)
    (else
      (Transformation|SetWorldRotation _sprite "0, 0, 0" false false)
      (Pawn|Input|AddMovementInput "-0.200000, 0, 0" 1.0 false)))
  (Utilities|FlowControl|Delay 2.9)
  (Variables|Default|SetNewVar_0 (not (Variables|Default|GetNewVar_0))))

(fn ConstructionScript)