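; Rope_Climb is a climbable rope or ladder actor that lets the Dave character climb while overlapping it.
; Its construction script stacks collision-free Paper2D sprites at a set spacing over the height between LadderStart and LadderEnd, then scales and centers a trigger Box from that height.
; Entering the Box sets Dave's CanClimb flag, and leaving clears it and calls EndofClimb.
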(event OnComponentBeginOverlap(Box)
  (params (OverlappedComponent :type Primitive%20Component%20Object%20Reference) (OtherActor :type Actor%20Object%20Reference) (OtherComp :type Primitive%20Component%20Object%20Reference) (OtherBodyIndex :type Integer) (bFromSweep :type Boolean) (SweepResult :type Hit%20Result%20Structure%20%28by%20ref%29))
  (bind _asdave (Utilities|Casting|CastToDave OtherActor))
  (Variables|/Game/NewSprites/Blueprints/Dave.Dave_C|SetbCanClimb _asdave true))

(event OnComponentEndOverlap(Box)
  (params (OverlappedComponent :type Primitive%20Component%20Object%20Reference) (OtherActor :type Actor%20Object%20Reference) (OtherComp :type Primitive%20Component%20Object%20Reference) (OtherBodyIndex :type Integer))
  (bind _asdave (Utilities|Casting|CastToDave OtherActor))
  (Variables|/Game/NewSprites/Blueprints/Dave.Dave_C|SetbCanClimb _asdave false)
  (Default|EndofClimb _asdave))

(event EventBeginPlay)

(event Collision|EventActorBeginOverlap
  (params (OtherActor :type Actor%20Object%20Reference)))

(event EventTick
  (params (DeltaSeconds :type Float%20%28single-precision%29)))

(fn ConstructionScript
  (bind _ladderstart (Variables|Default|GetLadderStart))
  (bind _ladderend (Variables|Default|GetLadderEnd))
  (bind _box (Variables|Default|GetBox))
  (bind _returnvalue (- _ladderend _ladderstart))
  (bind _returnvalue_2 (/ (.z _returnvalue) 2.0))
  (for _index (range 0 (Math|Float|Truncate (/ (.z _returnvalue) (Variables|Default|GetSeperation))))
    (bind _returnvalue_3 (AddComponent|AddPaperSpriteComponent false (Math|Transform|MakeTransform (Math|Vector|MakeVector 0.0 0.0 (* _index (Variables|Default|GetSeperation))) "0, 0, 0" "1,1,1")))
    (Rendering|Components|Sprite|SetSprite _returnvalue_3 (Variables|Default|GetLadderSprite))
    (Collision|SetCollisionEnabled _returnvalue_3 "NoCollision"))
  (Transformation|SetRelativeScale3D _box (Math|Vector|MakeVector 1.0 1.0 _returnvalue_2))
  (Transformation|SetRelativeLocation _box (Math|Vector|MakeVector 0.0 0.0 _returnvalue_2) false false))